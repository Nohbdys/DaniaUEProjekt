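; Exit door actor that tracks book-puzzle progress with six lights and opens once all six books are pressed.
; UpdateLight reads BooksPressedCounter from the first LevelDatabaseActor_Blueprint found in the level and turns one door light green per count through nested threshold checks.
; When the sixth light turns green it calls OpenDoor, which snaps the door from its BeginPlay rotation to an open yaw without animation.
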(event EventBeginPlay
  (Transformation|SetActorRotation "0.000000,-90.000000,0.000000"))

(fn ConstructionScript)

(fn OpenDoor
  (Transformation|SetActorRotation "0.000000,-190.000000, 0"))

(fn UpdateLight
  (bind _outactors (Actor|GetAllActorsOfClass "/Game/OurContent/BluePrints/LevelDatabaseActor_Blueprint.LevelDatabaseActor_Blueprint_C"))
  (if (> (Variables|/Game/OurContent/BluePrints/LevelDatabaseActor_Blueprint.LevelDatabaseActor_Blueprint_C|GetBooksPressedCounter (Utilities|Array|Get(acopy) _outactors)) 0)
    (Rendering|Components|Light|SetLightColor (Variables|/Script/Engine.Light|GetLightComponent (Variables|Default|GetDoorLight_1)) "(R=0.000000,G=1.000000,B=0.000000,A=1.000000)" true)
    (if (> (Variables|/Game/OurContent/BluePrints/LevelDatabaseActor_Blueprint.LevelDatabaseActor_Blueprint_C|GetBooksPressedCounter (Utilities|Array|Get(acopy) _outactors)) 1)
      (Rendering|Components|Light|SetLightColor (Variables|/Script/Engine.Light|GetLightComponent (Variables|Default|GetDoorLight_2)) "(R=0.000000,G=1.000000,B=0.000000,A=1.000000)" true)
      (if (> (Variables|/Game/OurContent/BluePrints/LevelDatabaseActor_Blueprint.LevelDatabaseActor_Blueprint_C|GetBooksPressedCounter (Utilities|Array|Get(acopy) _outactors)) 2)
        (Rendering|Components|Light|SetLightColor (Variables|/Script/Engine.Light|GetLightComponent (Variables|Default|GetDoorLight_3)) "(R=0.000000,G=1.000000,B=0.000000,A=1.000000)" true)
        (if (> (Variables|/Game/OurContent/BluePrints/LevelDatabaseActor_Blueprint.LevelDatabaseActor_Blueprint_C|GetBooksPressedCounter (Utilities|Array|Get(acopy) _outactors)) 3)
          (Rendering|Components|Light|SetLightColor (Variables|/Script/Engine.Light|GetLightComponent (Variables|Default|GetDoorLight_4)) "(R=0.000000,G=1.000000,B=0.000000,A=1.000000)" true)
          (if (> (Variables|/Game/OurContent/BluePrints/LevelDatabaseActor_Blueprint.LevelDatabaseActor_Blueprint_C|GetBooksPressedCounter (Utilities|Array|Get(acopy) _outactors)) 4)
            (Rendering|Components|Light|SetLightColor (Variables|/Script/Engine.Light|GetLightComponent (Variables|Default|GetDoorLight_5)) "(R=0.000000,G=1.000000,B=0.000000,A=1.000000)" true)
            (if (> (Variables|/Game/OurContent/BluePrints/LevelDatabaseActor_Blueprint.LevelDatabaseActor_Blueprint_C|GetBooksPressedCounter (Utilities|Array|Get(acopy) _outactors)) 5)
              (Rendering|Components|Light|SetLightColor (Variables|/Script/Engine.Light|GetLightComponent (Variables|Default|GetDoorLight_6)) "(R=0.000000,G=1.000000,B=0.000000,A=1.000000)" true)
              (CallFunction|OpenDoor))))))))