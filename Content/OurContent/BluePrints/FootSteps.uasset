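; FootSteps is an input-enabled Blueprint that plays wood footstep sounds while the W key is held.
; Pressing W plays the FootStep timeline from the start, and releasing it stops the timeline.
; The timeline's event track spawns the sound attached to the Audio component.
; A separate FootSteps function repeats that spawn but is not called in this graph.
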(event Custom|Play%20FootStep
  (Timeline|FootStep PlayFromStart
    (:FootSteps
      (Audio|SpawnSoundAttached "/Game/OurContent/Sounds/footsteps-on-wood__mp3cut_net2_.footsteps-on-wood__mp3cut_net2_" (Variables|Default|GetAudio)))))

(event Custom|Stop%20FootStep
  (Timeline|FootStep Stop
    (:FootSteps
      (Audio|SpawnSoundAttached "/Game/OurContent/Sounds/footsteps-on-wood__mp3cut_net2_.footsteps-on-wood__mp3cut_net2_" (Variables|Default|GetAudio)))))

(event EventTick
  (params (DeltaSeconds :type Float%20%28single-precision%29)))

(event EventBeginPlay
  (Input|EnableInput (Game|GetPlayerController 0)))

(event Input|KeyboardEvents|W
  (params (Key :type Key%20Structure))
  (:Pressed
    (CallFunction|PlayFootStep))
  (:Released
    (CallFunction|StopFootStep)))

(fn ConstructionScript)

(fn FootSteps
  (Audio|SpawnSoundAttached "/Game/OurContent/Sounds/footsteps-on-wood__mp3cut_net2_.footsteps-on-wood__mp3cut_net2_" (Variables|Default|GetAudio)))