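; An interactable piano book Actor that starts a piano lullaby when pressed.
; PressedPianoBook spawns the Rosemary's Baby lullaby attached to the root at low volume and lowered pitch, using the RockingChair attenuation settings.
; A PianoPlaying flag blocks repeat triggers and is never reset here, while the event graph and construction script add no logic.
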(event EventBeginPlay
  (|CallParentFunction) ; This node is disabled and will not be called.\nDrag off pins to build functionality.
)

(event Collision|EventActorBeginOverlap
  (params (OtherActor :type Actor%20Object%20Reference))
  (|CallParentFunction OtherActor) ; This node is disabled and will not be called.\nDrag off pins to build functionality.
)

(event EventTick
  (params (DeltaSeconds :type Float%20%28single-precision%29))
  (|CallParentFunction DeltaSeconds) ; This node is disabled and will not be called.\nDrag off pins to build functionality.
)

(fn ConstructionScript
  (|CallParentFunction))

(fn PressedPianoBook
  (if (not (Variables|Default|GetPianoPlaying))
    (Audio|SpawnSoundAttached "/Game/OurContent/Sounds/Lullaby_-_Rosemary_s_Baby__Piano___mp3cut_net_.Lullaby_-_Rosemary_s_Baby__Piano___mp3cut_net_" (Variables|Default|GetDefaultSceneRoot) "None" "0, 0, 0" "0, 0, 0" "KeepRelativeOffset" false 0.1 0.8 0.0 "/Game/OurContent/Sounds/RockingChair.RockingChair")
    (Variables|Default|SetPianoPlaying true)))