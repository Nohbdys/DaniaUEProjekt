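; Pennywise actor that plays an evil laugh sound effect once when its SoundTriggerScript fires OnSoundRequest.
; A DoOnce gate blocks repeat requests, and the sound spawns attached to the static mesh with lowered volume, slightly lowered pitch and attenuation settings from a variable.
; BeginPlay, overlap and Tick are disabled stubs, so the sound request is the only active logic.
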(event OnSoundRequest(SoundTriggerScript)
  (Utilities|FlowControl|DoOnce false
    (:Completed
      (Audio|SpawnSoundAttached "/Game/Content/Sounds/Evil_Laugh_Sound_Effect_mp3cut_net_.Evil_Laugh_Sound_Effect_mp3cut_net_" (Variables|Default|GetStaticMeshComponent) "None" "0, 0, 0" "0, 0, 0" "KeepRelativeOffset" false 0.2 0.95 0.0 (Variables|Default|GetNewVar_0)))))

(event EventBeginPlay
  (|CallParentFunction) ; This node is disabled and will not be called.\nDrag off pins to build functionality.
)

(event Collision|EventActorBeginOverlap
  (params (OtherActor :type Actor%20Object%20Reference))
  (|CallParentFunction OtherActor) ; This node is disabled and will not be called.\nDrag off pins to build functionality.
)

(event EventTick
  (params (DeltaSeconds :type Float%20%28single-precision%29))
  (|CallParentFunction DeltaSeconds) ; This node is disabled and will not be called.\nDrag off pins to build functionality.
)

(fn ConstructionScript
  (|CallParentFunction))