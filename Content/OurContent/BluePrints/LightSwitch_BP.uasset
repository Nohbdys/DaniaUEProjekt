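; LightSwitch_BP is a light switch that turns off an array of lights and records the press in the level database.
; ToggleLights, if LightsOn is set, increments BooksPressedCounter on the first LevelDatabaseActor_Blueprint found, zeroes each light's intensity and clears the flag.
; The branch that would turn the lights back on is disconnected, so the switch works only one way.
; The event graph and construction script are empty, leaving ToggleLights to external callers.
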(event EventBeginPlay)

(event Collision|EventActorBeginOverlap
  (params (OtherActor :type Actor%20Object%20Reference)))

(event EventTick
  (params (DeltaSeconds :type Float%20%28single-precision%29)))

(fn ConstructionScript)

(fn ToggleLights
  (if (Variables|Default|GetbLightsOn)
    (bind _outactors (Actor|GetAllActorsOfClass "/Game/OurContent/BluePrints/LevelDatabaseActor_Blueprint.LevelDatabaseActor_Blueprint_C"))
    (Variables|/Game/OurContent/BluePrints/LevelDatabaseActor_Blueprint.LevelDatabaseActor_Blueprint_C|SetBooksPressedCounter (Utilities|Array|Get(acopy) _outactors) (+ (Variables|/Game/OurContent/BluePrints/LevelDatabaseActor_Blueprint.LevelDatabaseActor_Blueprint_C|GetBooksPressedCounter (Utilities|Array|Get(acopy) _outactors)) 1))
    (for _array_element (Variables|Default|GetLights)
      (Rendering|Components|Light|SetIntensity (Variables|/Script/Engine.Light|GetLightComponent _array_element) 0.0)
      (Variables|Default|SetbLightsOn false))))