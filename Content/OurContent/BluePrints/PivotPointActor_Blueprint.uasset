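; PivotPointActor is a pivot actor that produces a rocking motion, apparently for a rocking chair given its sound.
; BeginPlay stores the root's world transform and spawns an attached, attenuated rocking-chair sound.
; Tick plays a timeline that lerps the root between that transform and a slight X offset with roll.
; When the timeline finishes, it restarts in the same direction, looping the motion.
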(event EventBeginPlay
  (bind _defaultsceneroot1 (Variables|Default|GetDefaultSceneRoot1))
  (Audio|SpawnSoundAttached "/Game/OurContent/Sounds/Rocking_Chair_Sound_Effect__mp3cut_net_.Rocking_Chair_Sound_Effect__mp3cut_net_" (Variables|Default|GetDefaultSceneRoot1) "None" "0, 0, 0" "0, 0, 0" "KeepRelativeOffset" false 1.0 1.0 0.0 "/Game/OurContent/Sounds/RockingChair.RockingChair")
  (bind _output_get (Variables|Default|SetInit%20Location (Transformation|GetWorldLocation _defaultsceneroot1)))
  (bind _output_get_2 (Variables|Default|SetInit%20rot (Transformation|GetWorldRotation _defaultsceneroot1))))

(event EventTick
  (params (DeltaSeconds :type Float%20%28single-precision%29))
  (bind (_direction _newtrack_0) (Timeline|Timeline Play)
    (:Update
      (bind _output_get (Variables|Default|SetMove%20to (Math|Vector|Lerp(Vector) (stale EventBeginPlay _output_get) (Math|Vector|MakeVector (+ (.X (Math|Vector|BreakVector (stale EventBeginPlay _output_get))) 2.2) (.Y (Math|Vector|BreakVector (stale EventBeginPlay _output_get))) (.Z (Math|Vector|BreakVector (stale EventBeginPlay _output_get)))) _newtrack_0)))
      (bind _output_get_2 (Variables|Default|SetRotate%20to (Math|Rotator|Lerp(Rotator) (stale EventBeginPlay _output_get_2) (Math|Rotator|MakeRotator (+ (.Roll (Math|Rotator|BreakRotator (stale EventBeginPlay _output_get_2))) -5.0) (.Pitch (Math|Rotator|BreakRotator (stale EventBeginPlay _output_get_2))) (.Yaw (Math|Rotator|BreakRotator (stale EventBeginPlay _output_get_2)))) _newtrack_0)))
      (Transformation|SetWorldLocationAndRotation (Variables|Default|GetDefaultSceneRoot1) _output_get _output_get_2 false false))
    (:Finished
      (switch Utilities|FlowControl|Switch|SwitchonETimelineDirection _direction
        (:Forward
          (Timeline|Timeline PlayFromStart))
        (:Backward
          (Timeline|Timeline ReverseFromEnd))))))

(fn ConstructionScript)